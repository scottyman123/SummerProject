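; BP_PushPull is a push/pull interactable box, currently a prototype that only reports player input and does not move.
; Overlapping its Fwd component sets CaninteractWBox on the third-person character cached at BeginPlay.
; While that flag and IsInteractingWBox are true, Tick reads ForwardBackwardAxis and prints forward, back or idle.
; A Speed/Direction graph holds an unused calculation choosing the cube's forward or right vector, scaled by DirectionSpeed.
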(event `self.ReceiveBeginPlay`
  (bind _returnvalue (`GameplayStatics.GetActorOfClass` "/Game/ThirdPerson/Blueprints/BP_ThirdPersonCharacter.BP_ThirdPersonCharacter_C"))
  (set `self.CharacterRef` _returnvalue))

(event `self.ReceiveTick`
  (params (DeltaSeconds :type "Float (single-precision)"))
  (bind _characterref (`self.CharacterRef`))
  (bind _forwardbackward_axis (`/Game/ThirdPerson/Blueprints/BP_ThirdPersonCharacter.ForwardBackward Axis` (`self.CharacterRef`)))
  (if (`/Game/ThirdPerson/Blueprints/BP_ThirdPersonCharacter.IsInteractingWBox?` _characterref)
    (if (`/Game/ThirdPerson/Blueprints/BP_ThirdPersonCharacter.CaninteractWBox?` _characterref)
      (`|ExecutionSequence`
        (:`then_0`
          (if (== _forwardbackward_axis 0.0)
            (`KismetSystemLibrary.PrintString` "is not moving forward or back" true true (struct :`R` 1.0 :`B` 0.055031 :`A` 1.0))
            (elif (>= _forwardbackward_axis 0.1)
              (`KismetSystemLibrary.PrintString` "is moving forward " true true (struct :`G` 1.0 :`B` 0.283917 :`A` 1.0))
              (else
                (`KismetSystemLibrary.PrintString` "is moving Back" true true (struct :`G` 1.0 :`B` 0.283917 :`A` 1.0))))))))))

(event `self.Fwd.OnComponentBeginOverlap`
  (params (OverlappedComponent :type "PrimitiveComponent Object Reference") (OtherActor :type "Actor Object Reference") (OtherComp :type "PrimitiveComponent Object Reference") (OtherBodyIndex :type Integer) (bFromSweep :type Boolean) (SweepResult :type "HitResult Structure (by ref)"))
  (`KismetSystemLibrary.PrintString` "Can interact" true true (struct :`R` 0.187448 :`G` 1.0 :`B` 0.024608 :`A` 1.0))
  (set `/Game/ThirdPerson/Blueprints/BP_ThirdPersonCharacter.CaninteractWBox?` true (`self.CharacterRef`)))

(event `self.Fwd.OnComponentEndOverlap`
  (params (OverlappedComponent :type "PrimitiveComponent Object Reference") (OtherActor :type "Actor Object Reference") (OtherComp :type "PrimitiveComponent Object Reference") (OtherBodyIndex :type Integer))
  (`KismetSystemLibrary.PrintString` "Cant interact" true true (struct :`R` 1.0 :`G` 0.009094 :`A` 1.0))
  (set `/Game/ThirdPerson/Blueprints/BP_ThirdPersonCharacter.CaninteractWBox?` false (`self.CharacterRef`)))

(fn `UserConstructionScript`)